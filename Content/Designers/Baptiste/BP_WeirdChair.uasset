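; BP_WeirdChair is an actor that endlessly animates the scale of its Mouth component, starting on BeginPlay.
; A FlipFlop alternates between one timeline played forward and a second played in reverse, each calling the Animation event again when finished.
; Both timelines lerp X and Z scale in opposite directions while Y stays fixed, giving a looping squash-and-stretch motion.
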(event Custom|Animation
  (Utilities|FlowControl|FlipFlop
    (:A
      (bind _newtrack_1 (Timeline|Timeline PlayFromStart)
        (:Update
          (Transformation|SetRelativeScale3D (Variables|Default|Getmouth) (Math|Vector|MakeVector (Math|Float|Lerp 1.0 0.85 _newtrack_1) 1.0 (Math|Float|Lerp 0.85 1.0 _newtrack_1))))
        (:Finished
          (CallFunction|Animation))))
    (:B
      (bind _newtrack_1_2 (Timeline|Timeline_0 ReverseFromEnd)
        (:Update
          (Transformation|SetRelativeScale3D (Variables|Default|Getmouth) (Math|Vector|MakeVector (Math|Float|Lerp 1.0 0.85 _newtrack_1_2) 1.0 (Math|Float|Lerp 0.85 1.0 _newtrack_1_2))))
        (:Finished
          (CallFunction|Animation))))))

(event EventBeginPlay
  (CallFunction|Animation))

(event Collision|EventActorBeginOverlap
  (params (OtherActor :type Actor%20Object%20Reference)))

(event EventTick
  (params (DeltaSeconds :type Float%20%28single-precision%29)))

(fn ConstructionScript)
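; BP_ClosetHiding is an interactable closet hiding spot that adds a visual effect when the player hides in it.
; Its Interact override runs the parent logic first, then checks PlayerHidden.
; If the player is hidden, it spawns the NS_Hiding_in_Closet Niagara system slightly above the actor's location.
; All other hiding behavior is left to the parent class, as the event graph holds only disabled default events.
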(event EventBeginPlay
  (|CallParentFunction) ; This node is disabled and will not be called.\nDrag off pins to build functionality.
)

(event Collision|EventActorBeginOverlap
  (params (OtherActor :type Actor%20Object%20Reference)))

(event EventTick
  (params (DeltaSeconds :type Float%20%28single-precision%29))
  (|CallParentFunction DeltaSeconds) ; This node is disabled and will not be called.\nDrag off pins to build functionality.
)

(fn ConstructionScript
  (|CallParentFunction))

(fn Interact
  (params (User :type Actor%20Object%20Reference))
  (|CallParentFunction User)
  (if (Variables|Default|GetPlayer%20Hidden)
    (Niagara|SpawnSystematLocation "/Game/Artists/04_VFX/NS_Hiding_in_Closet.NS_Hiding_in_Closet" (+ (Transformation|GetActorLocation) "0.000000,0.000000,10.000000"))))
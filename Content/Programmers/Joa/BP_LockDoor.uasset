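; Interactable hinged door that opens or closes on use unless locked, with a sound for each action.
; A dot product with the user's position picks the swing direction, and a timeline lerps the hinge yaw while door collision is off.
; The door closes when Alex or an enemy leaves the interact zone.
; Show and unshow events toggle a custom depth stencil value on the door mesh.
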(event OnComponentEndOverlap(InteractZoneCollision)
  (params (OverlappedComponent :type Primitive%20Component%20Object%20Reference) (OtherActor :type Actor%20Object%20Reference) (OtherComp :type Primitive%20Component%20Object%20Reference) (OtherBodyIndex :type Integer))
  (if (or (.bSuccess (Utilities|Casting|CastToBP_Alex OtherActor)) (.bSuccess (Utilities|Casting|CastToBP_Enemy OtherActor)))
    (CallFunction|CloseDoor)))

(event Custom|OnShow_Event
  (Rendering|SetCustomDepthStencilValue (Variables|Default|GetDoor) 3))

(event Custom|OnUnShow_Event
  (Rendering|SetCustomDepthStencilValue (Variables|Default|GetDoor) 0))

(event Custom|CloseDoor
  (bind _custom_hinge (Variables|Default|GetCustom_Hinge))
  (bind _relativerotation (Variables|/Script/Engine.SceneComponent|GetRelativeRotation _custom_hinge))
  (Audio|PlaySoundatLocation "/Game/Designers/Paul/SoundFX/Door/SC_Close_Door1_Cue.SC_Close_Door1_Cue" (+ (Transformation|GetActorLocation) "-850.000000,0.000000,1439.000000") "0, 0, 0" 1.0 1.0 0.0 "/Game/Programmers/Joa/Attenuation.Attenuation" 0 0 0)
  (Variables|Default|SetGoalRotation 0.0)
  (Variables|Default|SetStartPos (.yaw (Variables|/Script/Engine.SceneComponent|GetRelativeRotation (Variables|Default|GetCustom_Hinge))))
  (Variables|Default|SetOpen false)
  (Collision|SetCollisionEnabled (Variables|Default|GetDoor) "NoCollision")
  (bind _opening (Timeline|Timeline PlayFromStart)
    (:Update
      (Transformation|SetRelativeRotation _custom_hinge (Math|Rotator|MakeRotator (.roll _relativerotation) (.pitch _relativerotation) (Math|Float|Lerp (Variables|Default|GetStartPos) (Variables|Default|GetGoalRotation) _opening)) false false))
    (:Finished
      (Collision|SetCollisionEnabled (Variables|Default|GetDoor) "QueryOnly"))))

(event Custom|OpenDoor
  (params (GoalRot :type Float%20%28double-precision%29))
  (bind _custom_hinge (Variables|Default|GetCustom_Hinge))
  (bind _relativerotation (Variables|/Script/Engine.SceneComponent|GetRelativeRotation _custom_hinge))
  (Audio|PlaySoundatLocation "/Game/Designers/Paul/SoundFX/Door/SC_Open_Door_1_Cue.SC_Open_Door_1_Cue" (+ (Transformation|GetActorLocation) "-850.000000,0.000000,1439.000000") "0, 0, 0" 1.0 1.0 0.0 "/Game/Programmers/Joa/Attenuation.Attenuation" 0 0 0)
  (Variables|Default|SetGoalRotation GoalRot)
  (Variables|Default|SetStartPos (.yaw (Variables|/Script/Engine.SceneComponent|GetRelativeRotation (Variables|Default|GetCustom_Hinge))))
  (Variables|Default|SetOpen true)
  (Collision|SetCollisionEnabled (Variables|Default|GetDoor) "NoCollision")
  (bind _opening (Timeline|Timeline PlayFromStart)
    (:Update
      (Transformation|SetRelativeRotation _custom_hinge (Math|Rotator|MakeRotator (.roll _relativerotation) (.pitch _relativerotation) (Math|Float|Lerp (Variables|Default|GetStartPos) (Variables|Default|GetGoalRotation) _opening)) false false))
    (:Finished
      (Collision|SetCollisionEnabled (Variables|Default|GetDoor) "QueryOnly"))))

(event EventBeginPlay
  (|CallParentFunction)
  (EventDispatchers|BindEventtoOnShow (delegate Custom|OnShow_Event))
  (EventDispatchers|BindEventtoOnUnShow (delegate Custom|OnUnShow_Event)))

(event EventTick
  (params (DeltaSeconds :type Float%20%28single-precision%29))
  (|CallParentFunction DeltaSeconds) ; This node is disabled and will not be called.\nDrag off pins to build functionality.
)

(fn ConstructionScript
  (|CallParentFunction))

(fn Interact
  (params (User :type Actor%20Object%20Reference))
  (bind _returnvalue (Transformation|GetActorLocation))
  (bind _self self)
  (bind _returnvalue_2 (Transformation|GetActorRightVector _self))
  (bind _returnvalue_3 (Transformation|GetActorLocation User))
  (bind _returnvalue_4 (- _returnvalue_3 _returnvalue))
  (|CallParentFunction User)
  (if (not (Variables|Default|GetLocked))
    (if (Variables|Default|GetOpen)
      (CallFunction|CloseDoor)
      (else
        (CallFunction|OpenDoor (Math|Float|SelectFloat -9e+01 9e+01 (>= (Math|Vector2D|DotProduct(2D) (Math|Vector2D|MakeVector2D (.x _returnvalue_2) (.y _returnvalue_2)) (Math|Vector2D|MakeVector2D (.x _returnvalue_4) (.y _returnvalue_4))) 0.0)))))))
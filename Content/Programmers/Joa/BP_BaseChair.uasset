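; Base chair Blueprint for an interactable chair that can be reset to its starting placement.
; It records its location and rotation at BeginPlay and restores both on the Reset event.
; Interact runs the parent logic, then toggles collision on the chair model and interact zone together, using the zone's current collision state as the switch.
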(event Custom|Reset
  (Transformation|SetActorLocationAndRotation (Variables|Default|GetStartPos) (Variables|Default|GetStartRotation)))

(event EventBeginPlay
  (|CallParentFunction)
  (Variables|Default|SetStartPos (Transformation|GetActorLocation))
  (Variables|Default|SetStartRotation (Transformation|GetActorRotation)))

(event EventTick
  (params (DeltaSeconds :type Float%20%28single-precision%29))
  (|CallParentFunction DeltaSeconds) ; This node is disabled and will not be called.\nDrag off pins to build functionality.
)

(fn ConstructionScript
  (|CallParentFunction))

(fn Interact
  (params (User :type Actor%20Object%20Reference))
  (bind _interactzonecollision (Variables|Default|GetInteractZoneCollision))
  (bind _chairmodel (Variables|Default|GetChairModel))
  (|CallParentFunction User)
  (if (Utilities|Enum|Equal(Enum) (Collision|GetCollisionEnabled _interactzonecollision) "QueryOnly")
    (Collision|SetCollisionEnabled _interactzonecollision "NoCollision")
    (Collision|SetCollisionEnabled _chairmodel "NoCollision")
    (else
      (Collision|SetCollisionEnabled _interactzonecollision "QueryOnly")
      (Collision|SetCollisionEnabled _chairmodel "QueryAndPhysics"))))
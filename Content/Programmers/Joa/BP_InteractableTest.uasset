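; Test interactable Blueprint that toggles its own collision when interacted with.
; The Interact override calls the parent, then checks whether InteractZoneCollision is query-only.
; If so, it disables collision on both the zone and the Cube; otherwise it restores query-only on the zone and query-and-physics on the Cube.
; The event graph and construction script add no custom logic.
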(event EventBeginPlay
  (|CallParentFunction) ; This node is disabled and will not be called.\nDrag off pins to build functionality.
)

(event EventTick
  (params (DeltaSeconds :type Float%20%28single-precision%29))
  (|CallParentFunction DeltaSeconds) ; This node is disabled and will not be called.\nDrag off pins to build functionality.
)

(fn ConstructionScript
  (|CallParentFunction))

(fn Interact
  (bind _interactzonecollision (Variables|Default|GetInteractZoneCollision))
  (bind _cube (Variables|Default|GetCube))
  (|CallParentFunction)
  (if (Utilities|Enum|Equal(Enum) (Collision|GetCollisionEnabled _interactzonecollision) "QueryOnly")
    (Collision|SetCollisionEnabled _interactzonecollision "NoCollision")
    (Collision|SetCollisionEnabled _cube "NoCollision")
    (else
      (Collision|SetCollisionEnabled _interactzonecollision "QueryOnly")
      (Collision|SetCollisionEnabled _cube "QueryAndPhysics"))))
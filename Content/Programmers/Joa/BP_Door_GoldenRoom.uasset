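; Door Blueprint for the golden room that shows whether it is locked through its widget.
; The Lock event stores the Locked state, constructs either the lock widget or the standard interaction widget, and assigns it to the Widget component.
; The construction script only calls its parent, and the BeginPlay, overlap and Tick events are disabled.
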(event Custom|Lock
  (params (Lock :type Boolean))
  (Variables|Default|SetLocked Lock)
  (bind _returnvalue (Game|ConstructObjectfromClass (select Lock "/Game/Programmers/Common/WBP_Lock.WBP_Lock_C" "/Game/Programmers/Common/WBP_InteractionWidget.WBP_InteractionWidget_C")))
  (bind _asuser_widget (Utilities|Casting|CastToUserWidget _returnvalue))
  (UserInterface|SetWidget (Variables|Default|GetWidget) _asuser_widget))

(event EventBeginPlay
  (|CallParentFunction) ; This node is disabled and will not be called.\nDrag off pins to build functionality.
)

(event Collision|EventActorBeginOverlap
  (params (OtherActor :type Actor%20Object%20Reference)))

(event EventTick
  (params (DeltaSeconds :type Float%20%28single-precision%29))
  (|CallParentFunction DeltaSeconds) ; This node is disabled and will not be called.\nDrag off pins to build functionality.
)

(fn ConstructionScript
  (|CallParentFunction))
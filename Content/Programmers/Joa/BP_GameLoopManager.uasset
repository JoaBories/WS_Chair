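; Game loop manager for a two-phase chair-return objective, ending in a win screen.
; Chairs overlapping ChairRedeem snap onto their index-paired placeholders with confetti, sound and rumble; clearing all unlocks the door, reveals the golden placeholder and plays a cinematic.
; The golden phase accepts only GoldenChair, moves the manager itself to that placeholder, then plays the victory cinematic.
; Cinematics disable player input until their finished callback, which shows the win widget once Golden is false.
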(event OnComponentBeginOverlap(ChairRedeem)
  (params (OverlappedComponent :type Primitive%20Component%20Object%20Reference) (OtherActor :type Actor%20Object%20Reference) (OtherComp :type Primitive%20Component%20Object%20Reference) (OtherBodyIndex :type Integer) (bFromSweep :type Boolean) (SweepResult :type Hit%20Result%20Structure%20%28by%20ref%29))
  (bind _missinggoldenchair (Variables|Default|GetMissingGoldenChair))
  (bind _returnvalue (Transformation|GetActorTransform _missinggoldenchair))
  (Utilities|FlowControl|Delay 0.1)
  (bind _asbp_base_chair (Utilities|Casting|CastToBP_BaseChair OtherActor))
  (if (not (Variables|Default|GetGolden))
    (if (!= (Utilities|Array|FindItem (Variables|Default|GetChairs) _asbp_base_chair) -1)
      (CallFunction|PlacedChairFeedBack _asbp_base_chair)
      (Transformation|SetActorLocationAndRotation _asbp_base_chair (.location (Transformation|GetActorTransform (Utilities|Array|Get(acopy) (Variables|Default|GetChairsToRedeem) (Utilities|Array|FindItem (Variables|Default|GetChairs) _asbp_base_chair)))) (.rotation (Transformation|GetActorTransform (Utilities|Array|Get(acopy) (Variables|Default|GetChairsToRedeem) (Utilities|Array|FindItem (Variables|Default|GetChairs) _asbp_base_chair)))))
      (Default|BreakMe _asbp_base_chair)
      (Actor|DestroyActor (Utilities|Array|Get(acopy) (Variables|Default|GetChairsToRedeem) (Utilities|Array|FindItem (Variables|Default|GetChairs) _asbp_base_chair)))
      (Utilities|Array|RemoveIndex (Variables|Default|GetChairsToRedeem) (Utilities|Array|FindItem (Variables|Default|GetChairs) _asbp_base_chair))
      (Utilities|Array|RemoveIndex (Variables|Default|GetChairs) (Utilities|Array|FindItem (Variables|Default|GetChairs) _asbp_base_chair))
      (if (and (Utilities|Array|IsEmpty (Variables|Default|GetChairs)) (Utilities|Array|IsEmpty (Variables|Default|GetChairsToRedeem)))
        (Default|Lock (Variables|Default|GetDoorToLock) false)
        (Rendering|SetActorHiddenInGame (Variables|Default|GetMissingGoldenChair) false)
        (Variables|Default|SetGolden true)
        (CallFunction|PlayCinematic 1)))
    (elif (== _asbp_base_chair (Variables|Default|GetGoldenChair))
      (CallFunction|PlacedChairFeedBack _asbp_base_chair)
      (Transformation|SetActorLocationAndRotation (.location _returnvalue) (.rotation _returnvalue))
      (Default|BreakMe (Variables|Default|GetGoldenChair))
      (Actor|DestroyActor _missinggoldenchair)
      (Audio|PlaySound2D "/Game/Designers/Paul/SoundFX/Victory/SC_VictoryNoise.SC_VictoryNoise" 1.0 1.0 0.0 0 0)
      (CallFunction|PlayCinematic 2)
      (Variables|Default|SetGolden false))))

(event Custom|CinematicFinished
  (Input|EnableInput (Game|GetPlayerCharacter 0) (Game|GetPlayerController 0))
  (Widget|RemovefromParent (Variables|Default|GetCinematicWidget))
  (if (not (Variables|Default|GetGolden))
    (bind _returnvalue (Game|ConstructObjectfromClass "/Game/Programmers/Joa/Menus/WBP_Win.WBP_Win_C"))
    (UserInterface|Viewport|AddtoViewport _returnvalue 0)))

(event Custom|PlayCinematic
  (params (Index :type Integer))
  (Input|DisableInput (Game|GetPlayerCharacter 0) (Game|GetPlayerController 0))
  (bind _returnvalue (Game|ConstructObjectfromClass "/Game/Programmers/Joa/Menus/WBP_Cinematic.WBP_Cinematic_C"))
  (bind _output_get (Variables|Default|SetCinematicWidget _returnvalue))
  (UserInterface|Viewport|AddtoViewport _output_get 0)
  (EventDispatchers|BindEventtoFinished _output_get (delegate Custom|CinematicFinished))
  (Default|PlayCinematic _output_get Index))

(event EventBeginPlay
  (Default|Lock (Variables|Default|GetDoorToLock) true)
  (Rendering|SetActorHiddenInGame (Variables|Default|GetMissingGoldenChair) true))

(fn ConstructionScript)

(fn PlacedChairFeedBack
  (params (ActorLocation :type Actor%20Object%20Reference))
  (Niagara|SpawnSystematLocation "/Game/Artists/04_VFX/NS_Confetti.NS_Confetti" (+ (Transformation|GetActorLocation ActorLocation) "0.000000,0.000000,100.000000"))
  (Audio|PlaySoundatLocation "/Game/Designers/Paul/SoundFX/Chair/SC_PickUpGoodChair_1_Cue.SC_PickUpGoodChair_1_Cue" (+ (Transformation|GetActorLocation) "-850.000000,0.000000,1439.000000") "0, 0, 0" 1.0 1.0 0.0 "/Game/Programmers/Joa/Attenuation.Attenuation" 0 0 0)
  (Game|Feedback|ClientPlayForceFeedback (Game|GetPlayerController 0) "/Game/Designers/Paul/ForceFeedback/FF_GoodChairDrop.FF_GoodChairDrop" "None" false false false))
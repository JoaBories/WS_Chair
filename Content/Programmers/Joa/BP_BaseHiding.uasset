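; BP_BaseHiding is an interactable hiding spot for the player character, BP_Alex.
; Interact responds only to player 0, toggling Alex between Hide and UnHide based on the character's Hidden state and mirroring the result in PlayerHidden.
; OnShow and OnUnShow events, bound at BeginPlay, switch the static mesh's custom depth stencil value between 1 and 0.
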(event Custom|OnShow_Event
  (Rendering|SetCustomDepthStencilValue (Variables|Default|GetStaticMesh) 1))

(event Custom|OnUnShow_Event
  (Rendering|SetCustomDepthStencilValue (Variables|Default|GetStaticMesh) 0))

(event EventBeginPlay
  (|CallParentFunction)
  (EventDispatchers|BindEventtoOnShow (delegate Custom|OnShow_Event))
  (EventDispatchers|BindEventtoOnUnShow (delegate Custom|OnUnShow_Event)))

(event EventTick
  (params (DeltaSeconds :type Float%20%28single-precision%29))
  (|CallParentFunction DeltaSeconds) ; This node is disabled and will not be called.\nDrag off pins to build functionality.
)

(fn ConstructionScript
  (|CallParentFunction))

(fn Interact
  (params (User :type Actor%20Object%20Reference))
  (bind _returnvalue (Game|GetPlayerCharacter 0))
  (|CallParentFunction User)
  (if (== User _returnvalue)
    (bind _asbp_alex (Utilities|Casting|CastToBP_Alex _returnvalue))
    (if (Variables|/Game/Programmers/Joa/BP_Alex.BP_Alex_C|GetHidden _asbp_alex)
      (Default|UnHide _asbp_alex)
      (Variables|Default|SetPlayer%20Hidden false)
      (else
        (Default|Hide _asbp_alex)
        (Variables|Default|SetPlayer%20Hidden true)))))
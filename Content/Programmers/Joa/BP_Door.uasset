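; BP_Door is an interactable hinged door that toggles between open and closed.
; Interact picks a 90-degree swing direction from the dot product of the door's and user's forward vectors, or closes the door if open.
; OpenDoor and CloseDoor share a timeline that lerps the hinge's yaw from its current angle to the goal.
; Door collision is disabled during the swing, then set to QueryOnly.
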(event Custom|CloseDoor
  (bind _custom_hinge (Variables|Default|GetCustom_Hinge))
  (bind _relativerotation (Variables|/Script/Engine.SceneComponent|GetRelativeRotation _custom_hinge))
  (Variables|Default|SetGoalRotation 0.0)
  (Variables|Default|SetStartPos (.yaw (Variables|/Script/Engine.SceneComponent|GetRelativeRotation (Variables|Default|GetCustom_Hinge))))
  (Variables|Default|SetOpen false)
  (Collision|SetCollisionEnabled (Variables|Default|GetDoor) "NoCollision")
  (bind _opening (Timeline|Timeline PlayFromStart)
    (:Update
      (Transformation|SetRelativeRotation _custom_hinge (Math|Rotator|MakeRotator (.roll _relativerotation) (.pitch _relativerotation) (Math|Float|Lerp (Variables|Default|GetStartPos) (Variables|Default|GetGoalRotation) _opening)) false false))
    (:Finished
      (Collision|SetCollisionEnabled (Variables|Default|GetDoor) "QueryOnly"))))

(event Custom|OpenDoor
  (params (GoalRot :type Float%20%28double-precision%29))
  (bind _custom_hinge (Variables|Default|GetCustom_Hinge))
  (bind _relativerotation (Variables|/Script/Engine.SceneComponent|GetRelativeRotation _custom_hinge))
  (Variables|Default|SetGoalRotation GoalRot)
  (Variables|Default|SetStartPos (.yaw (Variables|/Script/Engine.SceneComponent|GetRelativeRotation (Variables|Default|GetCustom_Hinge))))
  (Variables|Default|SetOpen true)
  (Collision|SetCollisionEnabled (Variables|Default|GetDoor) "NoCollision")
  (bind _opening (Timeline|Timeline PlayFromStart)
    (:Update
      (Transformation|SetRelativeRotation _custom_hinge (Math|Rotator|MakeRotator (.roll _relativerotation) (.pitch _relativerotation) (Math|Float|Lerp (Variables|Default|GetStartPos) (Variables|Default|GetGoalRotation) _opening)) false false))
    (:Finished
      (Collision|SetCollisionEnabled (Variables|Default|GetDoor) "QueryOnly"))))

(event EventBeginPlay
  (|CallParentFunction) ; This node is disabled and will not be called.\nDrag off pins to build functionality.
)

(event EventTick
  (params (DeltaSeconds :type Float%20%28single-precision%29))
  (|CallParentFunction DeltaSeconds) ; This node is disabled and will not be called.\nDrag off pins to build functionality.
)

(fn ConstructionScript
  (|CallParentFunction))

(fn Interact
  (params (User :type Actor%20Object%20Reference))
  (bind _self self)
  (bind _returnvalue (Transformation|GetActorForwardVector _self))
  (bind _returnvalue_2 (Transformation|GetActorForwardVector User))
  (|CallParentFunction User)
  (if (Variables|Default|GetOpen)
    (CallFunction|CloseDoor)
    (else
      (CallFunction|OpenDoor (Math|Float|SelectFloat 9e+01 -9e+01 (>= (Math|Vector2D|DotProduct(2D) (Math|Vector2D|MakeVector2D (.x _returnvalue) (.y _returnvalue)) (Math|Vector2D|MakeVector2D (.x _returnvalue_2) (.y _returnvalue_2))) 0.0))))))
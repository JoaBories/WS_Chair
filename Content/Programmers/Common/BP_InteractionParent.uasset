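; BP_InteractionParent is a base interactable actor that shows a prompt widget when the player is in range.
; BeginPlay caches the BP_Alex player and sets the widget's initial visibility.
; InteractZoneCollision overlaps with the player toggle the widget and fire the OnShow and OnUnShow dispatchers.
; Interact is an empty hook, with its debug print and the widget's camera-facing rotation left disconnected.
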(event OnComponentBeginOverlap(InteractZoneCollision)
  (params (OverlappedComponent :type Primitive%20Component%20Object%20Reference) (OtherActor :type Actor%20Object%20Reference) (OtherComp :type Primitive%20Component%20Object%20Reference) (OtherBodyIndex :type Integer) (bFromSweep :type Boolean) (SweepResult :type Hit%20Result%20Structure%20%28by%20ref%29))
  (if (== OtherActor (Game|GetPlayerCharacter 0))
    (bind _output_get (Variables|Default|SetWidgetActivated true))
    (Rendering|SetVisibility (Variables|Default|GetWidget) _output_get false)
    (Default|CallOnShow)))

(event OnComponentEndOverlap(InteractZoneCollision)
  (params (OverlappedComponent :type Primitive%20Component%20Object%20Reference) (OtherActor :type Actor%20Object%20Reference) (OtherComp :type Primitive%20Component%20Object%20Reference) (OtherBodyIndex :type Integer))
  (if (== OtherActor (Game|GetPlayerCharacter 0))
    (bind _output_get (Variables|Default|SetWidgetActivated false))
    (Rendering|SetVisibility (Variables|Default|GetWidget) _output_get false)
    (Default|CallOnUnShow)))

(event EventTick
  (params (DeltaSeconds :type Float%20%28single-precision%29)))

(event EventBeginPlay
  (bind _asbp_alex (Utilities|Casting|CastToBP_Alex (Game|GetPlayerCharacter 0)))
  (Variables|Default|SetCharacter _asbp_alex)
  (Rendering|SetVisibility (Variables|Default|GetWidget) (Variables|Default|GetWidgetActivated) false))

(fn ConstructionScript)

(fn Interact
  (params (User :type Actor%20Object%20Reference)))